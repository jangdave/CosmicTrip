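; Game mode for CosmicVR that runs a timed round of about a minute and shows a game-over screen when time runs out.
; BeginPlay starts the background sound, creates the game-over and timer widgets, and displays only the timer.
; Tick accumulates elapsed time and, once it exceeds the limit, adds the game-over widget and shows the mouse cursor every frame, with no one-shot guard.
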(event `self.ReceiveBeginPlay`
  (`GameplayStatics.PlaySound2D` "/Game/CosmicVR/Sound_background_cosmicVR.Sound_background_cosmicVR" 1.0 1.0 0.0 null null)
  (set `self.timer` 61.0)
  (bind _returnvalue (`|CreateWidget` "/Game/CosmicVR/UI/WBP_GameOver.WBP_GameOver_C"))
  (set `self.gameover` _returnvalue)
  (bind _returnvalue_2 (`|CreateWidget` "/Game/CosmicVR/UI/WBP_Timer.WBP_Timer_C"))
  (bind _output_get (set `self.timerWidget` _returnvalue_2))
  (`UserWidget.AddToViewport` _output_get 0))

(event `self.ReceiveTick`
  (params (DeltaSeconds :type "Float (single-precision)"))
  (set `self.curtime` (+ DeltaSeconds (`self.curtime`)))
  (if (< (- (`self.timer`) (`self.curtime`)) 0.0)
    (`UserWidget.AddToViewport` (`self.gameover`) 0)
    (set `PlayerController.bShowMouseCursor` true (`GameplayStatics.GetPlayerController` 0))))

(fn `UserConstructionScript`)