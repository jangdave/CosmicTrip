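; BP_VTH is a player-controlled pawn with flight-style steering, driven by four input axes.
; MoveForward and MoveRight add movement input along the actor's forward and right vectors.
; Turn changes roll and yaw together for a banking effect, scaled by turn rates and delta time, with no auto-leveling.
; Pitch computes a rate-scaled target and eases toward it with FInterpTo, leaving roll and yaw untouched.
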(event `InputAxis|MoveForward`
  (params (AxisValue :type "Float (single-precision)"))
  ;[1 1 1] Movement
  (`self.AddMovementInput` (`self.GetActorForwardVector`) AxisValue))

(event `InputAxis|MoveRight`
  (params (AxisValue :type "Float (single-precision)"))
  ;[1 1 1] Movement
  (`self.AddMovementInput` (`self.GetActorRightVector`) AxisValue))

(event `InputAxis|Turn`
  (params (AxisValue :type "Float (single-precision)"))
  (bind _returnvalue (`GameplayStatics.GetWorldDeltaSeconds`))
  (bind (_returnvalue_roll _returnvalue_pitch _returnvalue_yaw) (`KismetMathLibrary.BreakRotator` (`self.K2_GetActorRotation`)))
  ;[1 1 1] Movement
  (`self.K2_SetActorRotation` (`KismetMathLibrary.MakeRotator` (+ _returnvalue_roll (* AxisValue (`self.RollTurnRate`) _returnvalue)) _returnvalue_pitch (+ _returnvalue_yaw (* AxisValue (`self.YawTurnRate`) _returnvalue)))))

(event `InputAxis|Pitch`
  (params (AxisValue :type "Float (single-precision)"))
  (bind _returnvalue (`GameplayStatics.GetWorldDeltaSeconds`))
  (bind (_returnvalue_roll _returnvalue_pitch _returnvalue_yaw) (`KismetMathLibrary.BreakRotator` (`self.K2_GetActorRotation`)))
  ;[1 1 1] Movement
  (bind _result (`/Engine/EditorBlueprintResources/StandardMacros.NegateFloat` AxisValue)
    (:`  `
      (bind _output_get (set `self.TargetFloat` (+ _returnvalue_pitch (* _result (`self.PitchTurnRate`) _returnvalue))))
      (`self.K2_SetActorRotation` (`KismetMathLibrary.MakeRotator` _returnvalue_roll (`KismetMathLibrary.FInterpTo` _returnvalue_pitch _output_get _returnvalue 3.0) _returnvalue_yaw)))))

(fn `UserConstructionScript`)